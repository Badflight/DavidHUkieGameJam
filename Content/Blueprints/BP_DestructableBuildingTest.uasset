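; Test destructible building that spawns a BP_Explosive at its Scene location, passes itself as BuildingRef and flags itself destroyed, immediately on BeginPlay.
; Tick also drains structural integrity into a widget, spawning another explosive and stopping tick at zero.
; ChangeOfIntegrity pauses decay by disabling tick and refreshes the widget, with a timer calling Restart Decay to resume.
; The widget reference setup and actor destruction are disconnected and never run.
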(event Custom|Spawn%20Explosive
  (bind _returnvalue (Game|SpawnActorfromClass "/Game/Blueprints/BP_Explosive.BP_Explosive_C" (Math|Transform|MakeTransform (Transformation|GetWorldLocation (Variables|Default|GetScene)) "0, 0, 0" "1.000000,1.000000,1.000000") "Undefined" "MultiplyWithRoot" 0 0))
  (Variables|/Game/Blueprints/BP_Explosive.BP_Explosive_C|SetBuilding%20Ref _returnvalue self)
  (Variables|Default|SetBuilding%20Destroyed true)
  (Utilities|FlowControl|Delay 1e+01))

(event Custom|Change%20Of%20Integrity
  (Utilities|Time|SetTimerbyFunctionName 0 "Restart Decay" 5.0)
  (Actor|Tick|SetActorTickEnabled false)
  (Development|PrintString "Event called")
  (Variables|/Game/Blueprints/Widget/WBP_BuildingInteg.WBP_BuildingInteg_C|SetIntegrity (Variables|Default|GetWidgetRef) (Variables|Default|GetStructureInteg)))

(event EventTick
  (params (DeltaSeconds :type Float%20%28single-precision%29))
  (Variables|Default|SetStructureInteg (- (Variables|Default|GetStructureInteg) (Variables|Gameplay|GetRateOfDecay)))
  (bind _output_get (Variables|/Game/Blueprints/Widget/WBP_BuildingInteg.WBP_BuildingInteg_C|SetIntegrity (Variables|Default|GetWidgetRef) (Variables|Default|GetStructureInteg)))
  (if (<= _output_get 0.0)
    (CallFunction|SpawnExplosive)
    (Actor|Tick|SetActorTickEnabled false)))

(event EventBeginPlay
  (CallFunction|SpawnExplosive))

(fn ConstructionScript)

(fn RestartDecay
  (Development|PrintString "Function called")
  (Actor|Tick|SetActorTickEnabled true))