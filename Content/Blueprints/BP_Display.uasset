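; BP_Display is an interactable display linked to a building, through which the player pays to increase that building's structural integrity.
; Interact reports a destroyed building, or opens WBP_UserPopup with cost and integrity arrays, disables character input and shows the cursor.
; OptionSelection deducts Money from the third-person character without an affordability check, raises the building's StructureInteg and calls ChangeOfIntegrity.
; BeginPlay prints a warning when BuildingRef is empty.
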(event EventBeginPlay
  (if (== (Variables|Default|GetBuildingRef) 0)
    (Development|PrintString (Utilities|String|Append (Utilities|GetDisplayName self) " is empty"))))

(event EventOptionSelection
  (params (Cost :type Float%20%28double-precision%29) (Integ%20increase :type Float%20%28double-precision%29))
  (bind _buildingref (Variables|Default|GetBuildingRef))
  (bind _asbp_third_person_character (Utilities|Casting|CastToBP_ThirdPersonCharacter (Game|GetPlayerCharacter 0)))
  (bind _output_get (Variables|Default|SetAs%20BP%20Third%20Person%20Character _asbp_third_person_character))
  (Variables|/Game/ThirdPerson/Blueprints/BP_ThirdPersonCharacter.BP_ThirdPersonCharacter_C|SetMoney _output_get (- (Variables|/Game/ThirdPerson/Blueprints/BP_ThirdPersonCharacter.BP_ThirdPersonCharacter_C|GetMoney _output_get) Cost))
  (Variables|/Game/Blueprints/BP_DestructableBuildingTest.BP_DestructableBuildingTest_C|SetStructureInteg _buildingref (+ (Variables|/Game/Blueprints/BP_DestructableBuildingTest.BP_DestructableBuildingTest_C|GetStructureInteg _buildingref) Integ%20increase))
  (Default|ChangeOfIntegrity _buildingref))

(event EventInteract
  (bind _returnvalue (Game|GetPlayerController 0))
  (if (Variables|/Game/Blueprints/BP_DestructableBuildingTest.BP_DestructableBuildingTest_C|GetBuilding%20Destroyed (Variables|Default|GetBuildingRef))
    (Development|PrintString "Building gone")
    (else
      (bind _returnvalue_2 (UserInterface|CreateWidget "/Game/Blueprints/WBP_UserPopup.WBP_UserPopup_C"))
      (Variables|/Game/Blueprints/WBP_UserPopup.WBP_UserPopup_C|SetDisplay%20Ref _returnvalue_2 self)
      (Variables|/Game/Blueprints/WBP_UserPopup.WBP_UserPopup_C|SetCost _returnvalue_2 (Variables|Default|GetCostFloarArray))
      (Variables|/Game/Blueprints/WBP_UserPopup.WBP_UserPopup_C|SetIntegratiy _returnvalue_2 (Variables|Default|GetIntegratityIncreaseArray))
      (UserInterface|Viewport|AddtoViewport _returnvalue_2 0)
      (Input|DisableInput (Game|GetPlayerCharacter 0) _returnvalue)
      (Variables|/Script/Engine.PlayerController|SetbShowMouseCursor _returnvalue true))))

(fn ConstructionScript)