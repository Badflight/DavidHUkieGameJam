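; BP_IncomeBuilding is a building that accumulates money for the player to collect.
; After a delay at start, Tick adds RateOfIncome to MoneyStored every frame, unscaled by delta time, and prints the total.
; Interact opens WBP_ShopPopup with the stored amount and a self reference, disabling character input and showing the cursor.
; Collection adds MoneyStored to the character's Money without clearing it, then pauses Tick until a timer re-enables it.
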(event Custom|Timer%20Reset
  (Actor|Tick|SetActorTickEnabled true))

(event EventBeginPlay
  (Utilities|FlowControl|Delay 2.0)
  (Actor|Tick|SetActorTickEnabled true))

(event EventTick
  (params (DeltaSeconds :type Float%20%28single-precision%29))
  (bind _output_get (Variables|Default|SetMoneyStored (+ (Variables|Default|GetMoneyStored) (Variables|Default|GetRateOfIncome))))
  (Development|PrintString (Utilities|String|ToString(Float) _output_get) true true "(R=0.000000,G=0.660000,B=1.000000,A=1.000000)" DeltaSeconds))

(event EventInteract
  (bind _returnvalue (Game|GetPlayerController 0))
  (bind _returnvalue_2 (UserInterface|CreateWidget "/Game/Blueprints/WBP_ShopPopup.WBP_ShopPopup_C"))
  (Variables|/Game/Blueprints/WBP_ShopPopup.WBP_ShopPopup_C|SetShopRef _returnvalue_2 self)
  (Variables|/Game/Blueprints/WBP_ShopPopup.WBP_ShopPopup_C|SetMoneyStoredWBP _returnvalue_2 (Variables|Default|GetMoneyStored))
  (UserInterface|Viewport|AddtoViewport _returnvalue_2 0)
  (Input|DisableInput (Game|GetPlayerCharacter 0) _returnvalue)
  (Variables|/Script/Engine.PlayerController|SetbShowMouseCursor _returnvalue true))

(event EventCollection
  (bind _asbp_third_person_character (Utilities|Casting|CastToBP_ThirdPersonCharacter (Game|GetPlayerCharacter 0)))
  (Variables|/Game/ThirdPerson/Blueprints/BP_ThirdPersonCharacter.BP_ThirdPersonCharacter_C|SetMoney _asbp_third_person_character (+ (Variables|/Game/ThirdPerson/Blueprints/BP_ThirdPersonCharacter.BP_ThirdPersonCharacter_C|GetMoney _asbp_third_person_character) (Variables|Default|GetMoneyStored)))
  (Utilities|Time|SetTimerbyEvent (delegate Custom|Timer%20Reset) 5.0)
  (Actor|Tick|SetActorTickEnabled false))

(fn ConstructionScript)